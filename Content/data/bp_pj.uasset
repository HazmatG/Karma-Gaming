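; bp_pj is a set of project helper functions for fetching the player character and game mode already cast to project types.
; GetPJPlayer casts player character 0 to bp_mc, while GetPJModeGNB and GetPJModeGS cast the current game mode to bpmode_gnb and bpmode_gs.
; Each function returns the typed reference only when its cast succeeds, with no failure handling.
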(fn `GetPJModeGNB`
  (returns (`AsBpmode Gnb` :type "/Game/scripts/player/bpmode_gnb Object Reference"))
  (bind _asbpmode_gnb (cast `/Game/scripts/player/bpmode_gnb` (`GameplayStatics.GetGameMode` null)))
  (return _asbpmode_gnb))

(fn `GetPJModeGS`
  (returns (`AsBpmode Gs` :type "/Game/scripts/player/bpmode_gs Object Reference"))
  (bind _asbpmode_gs (cast `/Game/scripts/player/bpmode_gs` (`GameplayStatics.GetGameMode` null)))
  (return _asbpmode_gs))

(fn `GetPJPlayer`
  (returns (`AsBp Mc` :type "/Game/scripts/player/bp_mc Object Reference"))
  (bind _asbp_mc (cast `/Game/scripts/player/bp_mc` (`GameplayStatics.GetPlayerCharacter` null)))
  (return _asbp_mc))